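; Main menu HUD that creates the loading screen, main menu and info widgets and handles start, quit and credits.
; On BeginPlay it adds all three to the viewport, with the info widget collapsed on top, shows the cursor and disables pawn input.
; StartGame fades the loading screen and opens LevelName through a done-fading callback.
; Credits toggles the info widget's visibility from its Menu flag.
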(event `self.ReceiveBeginPlay`
  (bind _returnvalue (`self.GetOwningPlayerController`))
  (bind _returnvalue_2 (`GameplayStatics.GetPlayerPawn` 0))
  ;[1 1 1] Construct Widget
  (`|ExecutionSequence`
    (:`then_0`
      (bind _returnvalue_3 (`|CreateWidget` "/Game/Blueprints/WB_LoadingScreen.WB_LoadingScreen_C" (`self.GetOwningPlayerController`)))
      (bind _output_get (set `self.LoadingScreen` _returnvalue_3))
      (`/Game/Blueprints/WB_LoadingScreen.SetFade` _output_get 0.0)
      (`UserWidget.AddToViewport` _output_get 90000))
    (:`then_1`
      (bind _returnvalue_4 (`|CreateWidget` "/Game/Blueprints/WB_MainMenu.WB_MainMenu_C" (`self.GetOwningPlayerController`)))
      (bind _output_get_2 (set `self.MainMenu` _returnvalue_4))
      (`UserWidget.AddToViewport` _output_get_2 0)
      (`WidgetBlueprintLibrary.SetInputMode_GameAndUIEx` _returnvalue null "DoNotLock" false)
      (set `PlayerController.bShowMouseCursor` true _returnvalue)
      (`/Engine/EditorBlueprintResources/StandardMacros.IsValid` _returnvalue_2
        (:`Is Valid`
          (`self.DisableInput` _returnvalue_2 _returnvalue))))
    (:`then_2`
      (bind _returnvalue_5 (`|CreateWidget` "/Game/Blueprints/WB_Info.WB_Info_C" (`self.GetOwningPlayerController`)))
      (bind _output_get_3 (set `self.InfoWidget` _returnvalue_5))
      (`Widget.SetVisibility` _output_get_3 "Collapsed")
      (`UserWidget.AddToViewport` _output_get_3 100))))

(event `/Game/Blueprints/BP_HUD_Interface.StartGame`
  ;[1 1 1] Start Game
  (if (!= (`self.LevelName`) "None")
    (bind _loadingscreen (`self.LoadingScreen`)
      (:`then`
        (`Widget.SetVisibility` _loadingscreen "Visible")
        (`/Game/Blueprints/WB_LoadingScreen.SetFade` _loadingscreen 1.0)
        (add `/Game/Blueprints/WB_LoadingScreen.DoneFading` _loadingscreen (delegate `LoadingLevel`)))
      (:`else`))))

(event `/Game/Blueprints/BP_HUD_Interface.QuitGame`
  ;[1 1 1] Quit Game
  (`KismetSystemLibrary.QuitGame` (`self.GetOwningPlayerController`) "Quit"))

(event `/Game/Blueprints/BP_HUD_Interface.Credits`
  (params (Menu :type Boolean))
  ;[1 1 1] Credits
  (if Menu
    (bind _infowidget (`self.InfoWidget`)
      (:`then`
        (`Widget.SetVisibility` _infowidget "Collapsed")
        (`WidgetBlueprintLibrary.SetInputMode_GameAndUIEx` (`self.GetOwningPlayerController`) _infowidget "DoNotLock" false))
      (:`else`))
    (else
      (bind _infowidget_2 (`self.InfoWidget`)
        (:`then`
          (`Widget.SetVisibility` _infowidget_2 "Visible")
          (`WidgetBlueprintLibrary.SetInputMode_GameAndUIEx` (`self.GetOwningPlayerController`) _infowidget_2 "DoNotLock" false))
        (:`else`)))))

(event `LoadingLevel`
  ;[1 1 1] Start Game
  (`GameplayStatics.OpenLevel` (`self.LevelName`)))

(fn `UserConstructionScript`)